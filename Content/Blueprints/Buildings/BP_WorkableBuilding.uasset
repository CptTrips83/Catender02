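; BP_WorkableBuilding is a building that farmer NPCs work on to produce pickup rewards.
; ProcessWorking runs the parent logic, converts a BP_Farmer's working progress into building progress, and calls the OnWorkDone dispatcher once the needed amount is reached.
; WorkDone spawns rewards and resets the building's progress.
; Each WorkRewards entry rolls its percent chance per count, spawning pickups at the building with a random X-axis offset.
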(event `self.ReceiveBeginPlay`
  (`parent.ReceiveBeginPlay`)
  (add `self.OnWorkDone` (`|CreateDelegate` :!event `WorkDone`)))

(event `self.ProcessWorking`
  (params (NPCCharacter :type "CTFriendlyNPCCharacter Object Reference"))
  (`|ExecutionSequence`
    (:`then_0`
      (`parent.ProcessWorking` NPCCharacter))
    (:`then_1`
      (bind _asbp_farmer (cast `/Game/Blueprints/Character/FriendlyNPC/Farmer/BP_Farmer` NPCCharacter))
      (if (`/Game/Blueprints/Character/FriendlyNPC/Farmer/BP_Farmer.HasWorkingProgress` _asbp_farmer)
        (`/Game/Blueprints/Character/FriendlyNPC/Farmer/BP_Farmer.ResetWorkingProgress` _asbp_farmer)
        (`/Engine/EditorBlueprintResources/StandardMacros.IncrementFloat` (`self.CurrentWorkProgress`))))
    (:`then_2`
      (if (>= (`self.CurrentWorkProgress`) (`self.NeededWorkProgress`))
        (bind _asbp_farmer_2 (cast `/Game/Blueprints/Character/FriendlyNPC/Farmer/BP_Farmer` NPCCharacter))
        (`self.OnWorkDone` _asbp_farmer_2)))))

(fn `ResetWorkingProgress`
  (set `self.CurrentWorkProgress` 0.0))

(fn `SpawnRewards`
  (locals (PickupClass :type "/Game/Blueprints/Pickups/BP_Pickup_BASE Class Reference") (SpawnChance :type "Float (double-precision)"))
  (bind _returnvalue (`self.GetTransform`))
  (for _array_element (`self.WorkRewards`)
    (set `local.PickupClass` (break `/Game/Blueprints/Structures/S_WorkReward` _array_element))
    (set `local.SpawnChance` (`.SpawnChance_8_F71C35A14D26658788B7B481BBA67D5A` (break `/Game/Blueprints/Structures/S_WorkReward` _array_element)))
    (bind _result (`/Engine/EditorBlueprintResources/StandardMacros.DecrementInt` (`.Count_5_985156BF4C3CBD61A283C3BB5EBDA339` (break `/Game/Blueprints/Structures/S_WorkReward` _array_element)))
      (:`  `
        (for _ (range (+ _result 1))
          (if (<= (`KismetMathLibrary.RandomFloatInRange` 0.0 100.0) (`local.SpawnChance`))
            (`|SpawnActorFromClass` (`local.PickupClass`) (`KismetMathLibrary.MakeTransform` (`KismetMathLibrary.MakeVector` (+ (`KismetMathLibrary.RandomFloatInRange` -30.0 30.0) (.x (.location _returnvalue))) (.y (.location _returnvalue)) (.z (.location _returnvalue))) (.rotation _returnvalue) (.scale _returnvalue)) "AlwaysSpawn" "MultiplyWithRoot" null null)))))))

(fn `UserConstructionScript`)

(fn `WorkDone`
  (params (Farmer :type "/Game/Blueprints/Character/FriendlyNPC/Farmer/BP_Farmer Object Reference"))
  (`self.SpawnRewards`)
  (`self.ResetWorkingProgress`))