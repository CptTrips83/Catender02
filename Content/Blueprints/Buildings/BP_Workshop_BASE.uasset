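; Base workshop building that stocks tools and uses them to turn kittens into cats of a configured NPC class.
; When active and at max level, interaction spends world resources to add a tool up to a cap, otherwise deferring to parent building logic.
; A kitten overlapping the construction-site box consumes a tool and is replaced by the spawned cat.
; Tool-count changes toggle both boxes' collision off and on to refresh overlaps.
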(event `self.ReceiveBeginPlay`
  (add `self.AvailableToolsChanged` (delegate `OnAvailableToolsChanged`)))

(event `OnAvailableToolsChanged` :!signature `self.AvailableToolsChanged`
  (params (OldValue :type Integer) (NewValue :type Integer))
  (`self.RefreshWorkshop`))

(event `self.ConstructionSiteBoxComponent.OnComponentBeginOverlap`
  (params (OverlappedComponent :type "PrimitiveComponent Object Reference") (OtherActor :type "Actor Object Reference") (OtherComp :type "PrimitiveComponent Object Reference") (OtherBodyIndex :type Integer) (bFromSweep :type Boolean) (SweepResult :type "HitResult Structure (by ref)"))
  (if (and (> (`self.AvailableTools`) 0) (`|EnumEquality` (`CTBuildingComponent.BuildingState` (`self.BuildingComponent`)) "Active"))
    (bind _asbp_kitten (cast `/Game/Blueprints/Character/FriendlyNPC/Kitten/BP_Kitten` OtherActor))
    (`self.UseTool` _asbp_kitten)))

(fn `AddTool`
  (locals (`Old Value` :type Integer))
  (bind _availabletools (`self.AvailableTools`))
  (if (< (`self.AvailableTools`) (`self.MaxTools`))
    (`self.PayResources`)
    (set `local.Old Value` _availabletools)
    (bind _result (`/Engine/EditorBlueprintResources/StandardMacros.IncrementInt` _availabletools)
      (:`  `
        (set `self.AvailableTools` _result)
        (`self.AvailableToolsChanged` (`local.Old Value`) _result)))))

(fn `CanInteract`
  (returns (ReturnValue :type Boolean))
  (bind _returnvalue (`parent.CanInteract`))
  (return (and (or _returnvalue (`|EnumEquality` (`CTBuildingComponent.GetBuildingState` (`self.BuildingComponent`)) "Active")) (< (`self.AvailableTools`) (`self.MaxTools`)))))

(fn `CheckResources`
  (returns (NewParam :type Boolean))
  (locals (HasRequiredResources :type Boolean :default true))
  (for _array_element (`self.NeededResources`)
    (if (not (`CTWorldResourceComponent.CheckResource` (`CTGameModeLevel.GetWorldResourceComponent` (`self.GetGameMode`)) (break `Resource` _array_element) (`.Amount` (break `Resource` _array_element))))
      (set `local.HasRequiredResources` false)))
  (return (`local.HasRequiredResources`)))

(fn `DestroyKitten`
  (params (Kitten :type "/Game/Blueprints/Character/FriendlyNPC/Kitten/BP_Kitten Object Reference"))
  (`self.K2_DestroyActor` Kitten))

(fn `GetNeededResourcesForInteraction`
  (returns (ReturnValue :type "Array of Resource Structure"))
  (bind _returnvalue (`parent.GetNeededResourcesForInteraction`))
  (if (`|EnumInequality` (`CTBuildingComponent.GetBuildingState` (`self.BuildingComponent`)) "Active")
    (return _returnvalue)
    (else
      (return (`self.NeededResources`)))))

(fn `HasTool`
  (returns (HasTool :type Boolean))
  (return (> (`self.AvailableTools`) 0)))

(fn `Interact`
  (params (OtherSortable :type "CTSortable Object Reference"))
  (bind _buildingcomponent (`self.BuildingComponent`))
  (if (and (`|EnumEquality` (`CTBuildingComponent.GetBuildingState` _buildingcomponent) "Active") (== (`CTBuildingComponent.GetCurrentBuildingLevel` _buildingcomponent) (`CTBuildingComponent.GetMaxBuildingLevel` _buildingcomponent)))
    (if (`self.CheckResources`)
      (`self.AddTool`))
    (else
      (`parent.Interact` (`local.OtherSortable`)))))

(fn `PayResources`
  (for _array_element (`self.NeededResources`)
    (`CTWorldResourceComponent.TrySubtractResourceAmount` (`CTGameModeLevel.GetWorldResourceComponent` (`self.GetGameMode`)) (break `Resource` _array_element) (`.Amount` (break `Resource` _array_element)))))

(fn `RefreshWorkshop`
  (`PrimitiveComponent.SetCollisionEnabled` (`self.InteractionBoxComponent`) "NoCollision")
  (`PrimitiveComponent.SetCollisionEnabled` (`self.InteractionBoxComponent`) "QueryOnly")
  (`PrimitiveComponent.SetCollisionEnabled` (`self.ConstructionSiteBoxComponent`) "NoCollision")
  (`PrimitiveComponent.SetCollisionEnabled` (`self.ConstructionSiteBoxComponent`) "QueryOnly"))

(fn `SpawnCat`
  (params (Location :type "Vector Structure"))
  (bind _returnvalue (`|SpawnActorFromClass` (`self.NPCClass`) (`KismetMathLibrary.MakeTransform` Location) "AlwaysSpawn" "MultiplyWithRoot" null null))
  (`/Engine/EditorBlueprintResources/StandardMacros.IsValid` _returnvalue
    (:`Is Valid`
      (`self.NewCatSpawned` _returnvalue))))

(fn `UserConstructionScript`)

(fn `UseTool`
  (params (Kitten :type "/Game/Blueprints/Character/FriendlyNPC/Kitten/BP_Kitten Object Reference"))
  (locals (OldValue :type Integer))
  (`self.SpawnCat` (`self.K2_GetActorLocation` Kitten))
  (`self.DestroyKitten` Kitten)
  (bind _result (`/Engine/EditorBlueprintResources/StandardMacros.DecrementInt` (`self.AvailableTools`))
    (:`  `
      (`self.AvailableToolsChanged` (`local.OldValue`) _result))))