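; Base building Blueprint that grants one unit of its ResourceType, which by its name serves as an unlock, when it becomes active.
; On BeginPlay it binds to the BuildingComponent's state-changed event.
; The BuildingActive handler adds the unit through the game mode's WorldResourceComponent whenever the new state is Active.
; It does not check the old state or remove the resource when leaving Active.
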(event `self.ReceiveBeginPlay`
  (`parent.ReceiveBeginPlay`)
  (add `CTBuildingComponent.OnBuildingStateChanged` (`self.BuildingComponent`) (`|CreateDelegate` :!event `BuildingActive`)))

(fn `BuildingActive`
  (params (Buildable :type "CTBuildable Object Reference") (OldState :type "EBuildingState Enum" :default "Invisible") (NewState :type "EBuildingState Enum" :default "Invisible"))
  (if (`|EnumEquality` NewState "Active")
    (`CTWorldResourceComponent.TryAddResourceAmount` (`CTGameModeLevel.WorldResourceComponent` (`self.GetGameMode`)) (`self.ResourceType`) 1)))

(fn `UserConstructionScript`)