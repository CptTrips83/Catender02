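; Nursing home building that accumulates waiting kittens over time and lets the player spend resources to recruit one as a spawned BP_Kitten.
; Tick re-arms a random-interval timer that adds a kitten, clamped to a maximum, and re-activates the building every frame (flagged inefficient).
; Interaction requires a waiting kitten and enough world resources.
; Count changes broadcast an event that toggles the sprite's child flipbooks, which are sorted just above the building.
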(event `self.ReceiveBeginPlay`
  (`parent.ReceiveBeginPlay`)
  (`|ExecutionSequence`
    (:`then_0`
      (`self.InitializeKittenFlipbooks`))
    (:`then_1`
      (add `self.KittenAmountChanged` (`|CreateDelegate` :!event `OnKittenAmountChanged`))
      (`self.OnSortingLayerChanged` "Background"))))

(event `self.ReceiveTick`
  (params (DeltaSeconds :type "Float (single-precision)"))
  (`parent.ReceiveTick` DeltaSeconds)
  (`self.StartSpawnTimer`)
  ;[1 1 1] TODO Ineffizent
  (`self.SetActive` true))

(fn `AddKittenToHome`
  (locals (OldAmount :type Integer))
  (bind _currentkittens (`self.CurrentKittens`))
  (set `local.OldAmount` _currentkittens)
  (bind _result (`/Engine/EditorBlueprintResources/StandardMacros.IncrementInt` _currentkittens)
    (:`  `
      (bind _output_get (set `self.CurrentKittens` (`KismetMathLibrary.Clamp` _result 0 (`self.MaxKittens`))))
      (`self.KittenAmountChanged` self (`local.OldAmount`) _output_get))))

(fn `CalcSpawnTime`
  (returns (SpawnTime :type "Float (double-precision)"))
  (return (`KismetMathLibrary.RandomFloatInRange` (`self.MinKittenSpawnTime`) (`self.MaxKittenSpawnTime`))))

(fn `CanInteract`
  (returns (ReturnValue :type Boolean))
  (return (> (`self.CurrentKittens`) 0)))

(fn `FeedKitten`
  (bind _returnvalue (`CTWorldResourceComponent.TrySubtractResources` (`CTGameModeLevel.WorldResourceComponent` (`self.GetGameMode`)) (`self.NeededResources`)))
  (if _returnvalue
    (`self.SpawnKitten`)
    (`self.RemoveKittenFromHome`)))

(fn `GetKittenFlipbooks`
  (returns (Flipbooks :type "Array of PaperFlipbookComponent Object Reference"))
  (locals (Result :type "Array of PaperFlipbookComponent Object Reference"))
  (return (`self.KittenFlipbooks`)))

(fn `GetNeededResourcesForInteraction`
  (returns (ReturnValue :type "Array of Resource Structure"))
  (`parent.GetNeededResourcesForInteraction`)
  (return (`self.NeededResources`)))

(fn `HandleSpawnTimer`
  (`KismetSystemLibrary.K2_ClearAndInvalidateTimerHandle` (`self.KittenSpawnTimerHamdle`))
  (`self.AddKittenToHome`))

(fn `InitializeKittenFlipbooks`
  (`KismetArrayLibrary.Array_Clear` (`self.KittenFlipbooks`))
  (for _array_element (`SceneComponent.GetChildrenComponents` (`self.Sprite`) false)
    (bind _aspaper_flipbook_component (cast `PaperFlipbookComponent` _array_element))
    (`/Engine/EditorBlueprintResources/StandardMacros.IsValid` _aspaper_flipbook_component
      (:`Is Valid`
        (`KismetArrayLibrary.Array_Add` (`self.KittenFlipbooks`) _aspaper_flipbook_component)))))

(fn `Interact`
  (params (OtherSortable :type "CTSortable Object Reference"))
  (`self.FeedKitten`))

(fn `OnKittenAmountChanged`
  (params (NursingHome :type "/Game/Blueprints/Buildings/NursingHome/BP_NursingHome Object Reference") (OldAmount :type Integer) (NewAmount :type Integer))
  (bind _flipbooks (`self.GetKittenFlipbooks`))
  (for _index (range (+ (`KismetArrayLibrary.Array_Length` _flipbooks) 1))
    (bind _output (`|GetArrayItem` _flipbooks _index))
    (`/Engine/EditorBlueprintResources/StandardMacros.IsValid` _output
      (:`Is Valid`
        (`SceneComponent.SetVisibility` _output (> (`local.NewAmount`) _index) false)))))

(fn `OnSortingLayerChanged`
  (params (OldSortingLayer :type "ESortingLayer Enum" :default "Background") (NewSortingLayer :type "ESortingLayer Enum" :default "Background"))
  (for _array_element (`self.GetKittenFlipbooks`)
    (`PrimitiveComponent.SetTranslucentSortPriority` _array_element (+ (`PrimitiveComponent.TranslucencySortPriority` (`self.Sprite`)) 1))))

(fn `RemoveKittenFromHome`
  (locals (OldAmount :type Integer))
  (bind _currentkittens (`self.CurrentKittens`))
  (set `local.OldAmount` _currentkittens)
  (bind _result (`/Engine/EditorBlueprintResources/StandardMacros.DecrementInt` _currentkittens)
    (:`  `
      (bind _output_get (set `self.CurrentKittens` (`KismetMathLibrary.Clamp` _result 0 (`self.MaxKittens`))))
      (`self.KittenAmountChanged` self (`local.OldAmount`) _output_get))))

(fn `SpawnKitten`
  (bind _returnvalue (`|SpawnActorFromClass` "/Game/Blueprints/Character/FriendlyNPC/Kitten/BP_Kitten.BP_Kitten_C" (`KismetMathLibrary.MakeTransform` (`self.K2_GetActorLocation`)) "AlwaysSpawn" "MultiplyWithRoot" null null))
  (`GameplayStatics.PlaySoundAtLocation` "/Game/SFX/Kitten/Kitten_Recruited_Cue.Kitten_Recruited_Cue" (`self.K2_GetActorLocation` _returnvalue) (struct) 1.0 1.0 0.0 null null null null))

(fn `StartSpawnTimer`
  (if (not (`KismetSystemLibrary.K2_IsValidTimerHandle` (`self.KittenSpawnTimerHamdle`)))
    (bind _returnvalue (`KismetSystemLibrary.K2_SetTimerDelegate` (`|CreateDelegate` :!event `HandleSpawnTimer`) (`self.CalcSpawnTime`)))
    (set `self.KittenSpawnTimerHamdle` _returnvalue)))

(fn `UserConstructionScript`)