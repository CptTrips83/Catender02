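; BP_Shop is a shop building that turns its lights on only while the building is in the Active state.
; On BeginPlay it binds to the BuildingComponent's state-changed event, which feeds SwitchLights to set the visibility of two point lights.
; ProcessWorking passes the NPC character straight to the parent implementation, adding no shop-specific work logic.
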(event `self.ReceiveBeginPlay`
  (add `CTBuildingComponent.OnBuildingStateChanged` (`self.BuildingComponent`) (`|CreateDelegate` :!event `OnBuildingStateChanged`)))

(event `self.ProcessWorking`
  (params (NPCCharacter :type "CTFriendlyNPCCharacter Object Reference"))
  (`parent.ProcessWorking` NPCCharacter))

(fn `OnBuildingStateChanged`
  (params (Buildable :type "CTBuildable Object Reference") (OldState :type "EBuildingState Enum" :default "Invisible") (NewState :type "EBuildingState Enum" :default "Invisible"))
  (`self.SwitchLights` (`|EnumEquality` NewState "Active")))

(fn `SwitchLights`
  (params (Visible :type Boolean))
  (`SceneComponent.SetVisibility` (`self.PointLight1`) Visible false)
  (`SceneComponent.SetVisibility` (`self.PointLight`) (`local.Visible`) false))

(fn `UserConstructionScript`)