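; Base Blueprint for destroyable objects, filed under Buildings/Trees, that drops gold when destroyed.
; On BeginPlay it binds to its BuildingComponent's state-change event, with CheckForDestruction treating a transition into Invisible as destruction.
; SpawnGold then spawns a BP_Gold at the actor's location and launches it upward with a random sideways X velocity via a mass-independent impulse.
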(event `self.ReceiveBeginPlay`
  (add `CTBuildingComponent.OnBuildingStateChanged` (`self.BuildingComponent`) (`|CreateDelegate` :!event `CheckForDestruction`)))

(event `CheckForDestruction`
  (params (Buildable :type "CTBuildable Object Reference") (OldState :type "EBuildingState Enum" :default "Invisible") (NewState :type "EBuildingState Enum" :default "Invisible"))
  (if (and (`|EnumInequality` OldState "Invisible") (`|EnumEquality` NewState "Invisible"))
    (`self.SpawnGold`)))

(event `SpawnGold`
  (bind _returnvalue (`|SpawnActorFromClass` "/Game/Blueprints/Pickups/BP_Gold.BP_Gold_C" (`KismetMathLibrary.MakeTransform` (`self.K2_GetActorLocation`)) "AlwaysSpawn" "MultiplyWithRoot" null null))
  (`PrimitiveComponent.AddImpulse` (`Character.CapsuleComponent` _returnvalue) (+ (`KismetMathLibrary.MakeVector` (`KismetMathLibrary.Conv_IntToDouble` (`KismetMathLibrary.RandomIntegerInRange` -100 100))) (* (0.0 0.0 1.0) 300.0)) "None" true))

(fn `UserConstructionScript`)