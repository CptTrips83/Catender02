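; BP_Wall is a damageable wall building in the cat level that reacts to the day/night cycle.
; AddDamage accumulates clamped damage, broadcasts changes and triggers destruction through the BuildingComponent once the hit point check passes.
; At day, critically damaged walls return to Construction state, while lighter damage is simply cleared.
; Destruction resets damage and notifies the world archer component through a tower state-change call; a helper toggles the point light.
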(event `self.ReceiveBeginPlay`
  (`|ExecutionSequence`
    (:`then_0`
      (bind _asgm_cat_level (cast `/Game/Blueprints/GameModes/GM_CatLevel` (`GameplayStatics.GetGameMode`)))
      (add `CTWorldDayTimeComponent.OnDayNightChanged` (`CTGameModeLevel.GetWorldDayTimeComponent` _asgm_cat_level) (`|CreateDelegate` :!event `DayTimeChanged`)))
    (:`then_1`
      (add `self.OnWallDestroyed` (`|CreateDelegate` :!event `WallDestroyed`)))))

(fn `AddDamage`
  (params (Damage :type "Float (double-precision)"))
  (locals (`Old Damage` :type "Float (double-precision)" :default 0.0))
  (bind _currentdamage (`self.CurrentDamage`))
  (bind _returnvalue (+ (`local.Damage`) _currentdamage))
  (set `local.Old Damage` _currentdamage)
  (bind _output_get (set `self.CurrentDamage` (`KismetMathLibrary.FClamp` _returnvalue 0.0 (`self.HitPoints`))))
  (`self.OnDamageChanged` self (`local.Old Damage`) _output_get)
  (if (>= _returnvalue (`self.HitPoints`))
    (`self.DestroyWall`)))

(fn `CallWorldArcherComponent`
  (bind _asgm_cat_level (cast `/Game/Blueprints/GameModes/GM_CatLevel` (`self.GetGameMode`)))
  (`/Game/Blueprints/Components/BP_WorldArcher.TowerBuildingStateChanged` (`/Game/Blueprints/GameModes/GM_CatLevel.World Archer Component` _asgm_cat_level) null "Invisible" "Invisible"))

(fn `CanInteract`
  (returns (ReturnValue :type Boolean))
  (bind _returnvalue (`parent.CanInteract`))
  (return _returnvalue))

(fn `DayTimeChanged`
  (params (OldValue :type Integer) (NewValue :type Integer) (OldIsDay :type Boolean) (NewIsDay :type Boolean))
  (if NewIsDay
    (if (>= (`self.CurrentDamage`) (* (`self.HitPoints`) (`self.CriticalDamagePercentage`)))
      (`self.RebuildWall`)
      (else
        (`self.ResetWallDamage`)))))

(fn `DestroyWall`
  (`self.OnWallDestroyed` self)
  (`CTBuildingComponent.SetBuildingState` (`self.BuildingComponent`) "Destroyed")
  (`self.ResetWallDamage`))

(fn `GetCurrentDamage`
  (returns (CurrentDamage :type "Float (double-precision)"))
  (return (`self.CurrentDamage`)))

(fn `GetHitPoints`
  (returns (CurrentDamage :type "Float (double-precision)"))
  (return (`self.HitPoints`)))

(fn `Interact`
  (params (OtherSortable :type "CTSortable Object Reference"))
  (`parent.Interact` OtherSortable))

(fn `IsCriticalDamaged`
  (returns (IsDamaged :type Boolean))
  (return (>= (`self.CurrentDamage`) (* (`self.HitPoints`) (`self.CriticalDamagePercentage`)))))

(fn `RebuildWall`
  (`CTBuildingComponent.SetBuildingState` (`self.BuildingComponent`) "Construction")
  (`self.ResetWallDamage`))

(fn `ResetWallDamage`
  (`self.OnDamageChanged` self (`self.CurrentDamage`))
  (set `self.CurrentDamage` 0.0))

(fn `UpdateLights`
  (params (IsVisible :type Boolean))
  (`SceneComponent.SetVisibility` (`self.PointLight`) IsVisible false))

(fn `UserConstructionScript`)

(fn `WallDestroyed`
  (params (Target :type "/Game/Blueprints/Buildings/Wall/BP_Wall Object Reference"))
  (`self.CallWorldArcherComponent`))