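; Tool stand building piece that shows how many tools its owning workshop has available, using four flipbook sprites.
; When the owning workshop is set, it binds to the workshop's tool-count change event, gathers the sprites and picks their flipbook by the workshop's NPC class.
; Count changes toggle sprite visibility by index.
; Sprite sort priority is offset from the workshop's sprite, ignoring the layer arguments.
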(event `self.ReceiveBeginPlay`)

(event `AvailableToolsChanged`
  (params (OldValue :type Integer) (NewValue :type Integer))
  (`self.SetToolAmount` NewValue))

(fn `GetSpriteComponents`
  (`KismetArrayLibrary.Array_Add` (`self.Sprites`) (`self.Tool1`))
  (`KismetArrayLibrary.Array_Add` (`self.Sprites`) (`self.Tool2`))
  (`KismetArrayLibrary.Array_Add` (`self.Sprites`) (`self.Tool3`))
  (`KismetArrayLibrary.Array_Add` (`self.Sprites`) (`self.Tool4`))
  (`self.SetToolsSortingLayer` "Background"))

(fn `SetOwningWorkshop`
  (params (OwningWorkshop :type "/Game/Blueprints/Buildings/Workshop/BP_Workshop_BASE Object Reference"))
  (set `self.OwningWorkshop` OwningWorkshop)
  (`|ExecutionSequence`
    (:`then_0`
      (add `/Game/Blueprints/Buildings/Workshop/BP_Workshop_BASE.AvailableToolsChanged` (`self.OwningWorkshop`) (`|CreateDelegate` :!event `AvailableToolsChanged`))
      (`self.GetSpriteComponents`)
      (`self.SetSprites`))))

(fn `SetSprites`
  (set `self.ToolSprite` (`BlueprintMapLibrary.Map_Find` (`self.ToolSprites`) (`/Game/Blueprints/Buildings/Workshop/BP_Workshop_BASE.NPCClass` (`self.OwningWorkshop`))))
  (for _array_element (`self.Sprites`)
    (`PaperFlipbookComponent.SetFlipbook` _array_element (`self.ToolSprite`))))

(fn `SetToolAmount`
  (params (Amount :type Integer))
  (for (_array_element _array_index) (`self.Sprites`)
    (`SceneComponent.SetVisibility` _array_element (< _array_index (`local.Amount`)) false)))

(fn `SetToolsSortingLayer`
  (params (OldSortingLayer :type "ESortingLayer Enum" :default "Background") (NewSortingLayer :type "ESortingLayer Enum" :default "Background"))
  (for _array_element (`self.Sprites`)
    (`PrimitiveComponent.SetTranslucentSortPriority` _array_element (+ (`PrimitiveComponent.TranslucencySortPriority` (`PaperCharacter.Sprite` (`self.OwningWorkshop`))) 3))))

(fn `UserConstructionScript`)