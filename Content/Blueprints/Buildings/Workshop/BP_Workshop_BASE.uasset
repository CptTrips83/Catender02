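; Base workshop building that turns kittens into NPC cats of a configurable class using purchased tools.
; When active and fully upgraded, interaction spends resources to stock tools, and an overlapping kitten consumes one, being destroyed as a cat spawns.
; Tool count changes toggle box collisions to refresh overlaps.
; HQ level unlocks construction, while building state and sorting layer drive tool stand and vendor visuals.
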(event `self.ReceiveBeginPlay`
  (`|ExecutionSequence`
    (:`then_0`
      (bind _asgm_cat_level (cast `/Game/Blueprints/GameModes/GM_CatLevel` (`GameplayStatics.GetGameMode`)))
      (add `CTBuildingComponent.OnBuildingStateChanged` (`CTBuildable.BuildingComponent` (`CTGameModeLevel.GetBuildingHQ` _asgm_cat_level)) (`|CreateDelegate` :!event `OnHQBuildingStateChanged`))
      (add `CTBuildingComponent.OnBuildingStateChanged` (`self.BuildingComponent`) (`|CreateDelegate` :!event `OnOwnBuildingStateChanged`))
      (add `CTSortingComponent.OnSortingLayerChanged` (`self.GetSortingComponent`) (`|CreateDelegate` :!event `OnSortingLayerChanged`))
      (`self.OnSortingLayerChanged` "Background"))
    (:`then_1`
      (add `self.AvailableToolsChanged` (delegate `OnAvailableToolsChanged`)))))

(event `OnAvailableToolsChanged` :!signature `self.AvailableToolsChanged`
  (params (OldValue :type Integer) (NewValue :type Integer))
  (`self.RefreshWorkshop`))

(event `self.ConstructionSiteBoxComponent.OnComponentBeginOverlap`
  (params (OverlappedComponent :type "PrimitiveComponent Object Reference") (OtherActor :type "Actor Object Reference") (OtherComp :type "PrimitiveComponent Object Reference") (OtherBodyIndex :type Integer) (bFromSweep :type Boolean) (SweepResult :type "HitResult Structure (by ref)"))
  (if (and (> (`self.AvailableTools`) 0) (`|EnumEquality` (`CTBuildingComponent.BuildingState` (`self.BuildingComponent`)) "Active"))
    (bind _asbp_kitten (cast `/Game/Blueprints/Character/FriendlyNPC/Kitten/BP_Kitten` OtherActor))
    (`self.UseTool` _asbp_kitten)))

(fn `AddTool`
  (locals (`Old Value` :type Integer))
  (bind _availabletools (`self.AvailableTools`))
  (if (< (`self.AvailableTools`) (`self.MaxTools`))
    (`self.PayResources`)
    (set `local.Old Value` _availabletools)
    (bind _result (`/Engine/EditorBlueprintResources/StandardMacros.IncrementInt` _availabletools)
      (:`  `
        (set `self.AvailableTools` _result)
        (`self.AvailableToolsChanged` (`local.Old Value`) _result)))))

(fn `CanInteract`
  (returns (ReturnValue :type Boolean))
  (`parent.CanInteract`)
  (return (and (`|EnumEquality` (`CTBuildingComponent.GetBuildingState` (`self.BuildingComponent`)) "Active") (< (`self.AvailableTools`) (`self.MaxTools`)))))

(fn `CheckResources`
  (returns (NewParam :type Boolean))
  (locals (HasRequiredResources :type Boolean :default true))
  (for _array_element (`self.NeededResources`)
    (if (not (`CTWorldResourceComponent.CheckResource` (`CTGameModeLevel.GetWorldResourceComponent` (`self.GetGameMode`)) (break `Resource` _array_element) (`.Amount` (break `Resource` _array_element))))
      (set `local.HasRequiredResources` false)))
  (return (`local.HasRequiredResources`)))

(fn `DestroyKitten`
  (params (Kitten :type "/Game/Blueprints/Character/FriendlyNPC/Kitten/BP_Kitten Object Reference"))
  (`self.K2_DestroyActor` Kitten))

(fn `GetNeededResourcesForInteraction`
  (returns (ReturnValue :type "Array of Resource Structure"))
  (bind _returnvalue (`parent.GetNeededResourcesForInteraction`))
  (if (`|EnumInequality` (`CTBuildingComponent.GetBuildingState` (`self.BuildingComponent`)) "Active")
    (return _returnvalue)
    (else
      (return (`self.NeededResources`)))))

(fn `HasTool`
  (returns (HasTool :type Boolean))
  (return (> (`self.AvailableTools`) 0)))

(fn `Interact`
  (params (OtherSortable :type "CTSortable Object Reference"))
  (bind _buildingcomponent (`self.BuildingComponent`))
  (if (and (`|EnumEquality` (`CTBuildingComponent.GetBuildingState` _buildingcomponent) "Active") (== (`CTBuildingComponent.GetCurrentBuildingLevel` _buildingcomponent) (`CTBuildingComponent.GetMaxBuildingLevel` _buildingcomponent)))
    (if (`self.CheckResources`)
      (`self.AddTool`)
      (`GameplayStatics.PlaySoundAtLocation` "/Game/SFX/King/King_Recruit_Cue.King_Recruit_Cue" (`self.K2_GetActorLocation`) (struct) 1.0 1.0 0.0 null null null null))
    (else
      (`parent.Interact` (`local.OtherSortable`)))))

(fn `OnHQBuildingStateChanged`
  (params (Buildable :type "CTBuildable Object Reference") (OldState :type "EBuildingState Enum" :default "Invisible") (NewState :type "EBuildingState Enum" :default "Invisible"))
  (if (and (`|EnumInequality` (`CTBuildingComponent.GetBuildingState` (`self.BuildingComponent`)) "Active") (`|EnumEquality` NewState "Active"))
    (if (>= (`CTBuildingComponent.CurrentLevel` (`CTBuildable.BuildingComponent` (`local.Buildable`))) (`self.HQLevelNeeded`))
      (`CTBuildingComponent.SetBuildingState` (`self.BuildingComponent`) "Construction"))))

(fn `OnOwnBuildingStateChanged`
  (params (Buildable :type "CTBuildable Object Reference") (OldState :type "EBuildingState Enum" :default "Invisible") (NewState :type "EBuildingState Enum" :default "Invisible"))
  (`SceneComponent.SetVisibility` (`self.ToolStand`) (select `EBuildingState` (`local.NewState`) :`Active` true) false)
  (`SceneComponent.SetVisibility` (`self.VendorSprite`) (select `EBuildingState` (`local.NewState`) :`Active` true) false))

(fn `OnSortingLayerChanged`
  (params (OldSortingLayer :type "ESortingLayer Enum" :default "Background") (NewSortingLayer :type "ESortingLayer Enum" :default "Background"))
  (bind _asbp_toolstand (cast `/Game/Blueprints/Buildings/Workshop/BP_Toolstand` (`ChildActorComponent.ChildActor` (`self.ToolStand`))))
  (`PrimitiveComponent.SetTranslucentSortPriority` (`PaperCharacter.Sprite` _asbp_toolstand) (+ (`PrimitiveComponent.TranslucencySortPriority` (`self.Sprite`)) 2))
  (`PrimitiveComponent.SetTranslucentSortPriority` (`self.VendorSprite`) (+ (`PrimitiveComponent.TranslucencySortPriority` (`self.Sprite`)) 1)))

(fn `PayResources`
  (for _array_element (`self.NeededResources`)
    (`CTWorldResourceComponent.TrySubtractResourceAmount` (`CTGameModeLevel.GetWorldResourceComponent` (`self.GetGameMode`)) (break `Resource` _array_element) (`.Amount` (break `Resource` _array_element)))))

(fn `RefreshWorkshop`
  (`PrimitiveComponent.SetCollisionEnabled` (`self.InteractionBoxComponent`) "NoCollision")
  (`PrimitiveComponent.SetCollisionEnabled` (`self.InteractionBoxComponent`) "QueryOnly")
  (`PrimitiveComponent.SetCollisionEnabled` (`self.ConstructionSiteBoxComponent`) "NoCollision")
  (`PrimitiveComponent.SetCollisionEnabled` (`self.ConstructionSiteBoxComponent`) "QueryOnly"))

(fn `SpawnCat`
  (params (Location :type "Vector Structure"))
  (bind _returnvalue (`|SpawnActorFromClass` (`self.NPCClass`) (`KismetMathLibrary.MakeTransform` Location) "AlwaysSpawn" "MultiplyWithRoot" null null))
  (`/Engine/EditorBlueprintResources/StandardMacros.IsValid` _returnvalue
    (:`Is Valid`
      (`self.NewCatSpawned` _returnvalue))))

(fn `UserConstructionScript`)

(fn `UseTool`
  (params (Kitten :type "/Game/Blueprints/Character/FriendlyNPC/Kitten/BP_Kitten Object Reference"))
  (locals (OldValue :type Integer))
  (`self.SpawnCat` (`SceneComponent.K2_GetComponentLocation` (`self.CatSpawner`)))
  (`self.DestroyKitten` Kitten)
  (bind _result (`/Engine/EditorBlueprintResources/StandardMacros.DecrementInt` (`self.AvailableTools`))
    (:`  `
      (`self.AvailableToolsChanged` (`local.OldValue`) _result))))