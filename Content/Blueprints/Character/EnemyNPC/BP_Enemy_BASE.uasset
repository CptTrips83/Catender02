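; Base enemy NPC that advances on the player's HQ along the X axis and attacks walls in its path.
; Tick drives AI movement and a delay-gated attack; overlapping a wall stops movement and enables capsule physics.
; Attacks play a jump animation, launch the capsule with an HQ-directed impulse, then damage the stored wall.
; Projectile overlaps reduce hitpoints, triggering hit animations or a depletion event, whose handler destroys the actor.
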(event `self.ReceiveBeginPlay`
  (add `self.CurrentHitpointsDepleted` (`|CreateDelegate` :!event `OnCurrentHitpointsDepleted`)))

(event `self.ReceiveTick`
  (params (DeltaSeconds :type "Float (single-precision)"))
  (`self.MoveToHQ`)
  (`self.Attack`))

(event `self.HitCollision.OnComponentBeginOverlap`
  (params (OverlappedComponent :type "PrimitiveComponent Object Reference") (OtherActor :type "Actor Object Reference") (OtherComp :type "PrimitiveComponent Object Reference") (OtherBodyIndex :type Integer) (bFromSweep :type Boolean) (SweepResult :type "HitResult Structure (by ref)"))
  (bind _asbp_projectile_base (cast `/Game/Blueprints/Projectiles/BP_Projectile_BASE` OtherActor))
  (`self.AddDamage` (`CTProjectile.GetDamage` _asbp_projectile_base)))

(event `self.WallDetector.OnComponentBeginOverlap`
  (params (OverlappedComponent :type "PrimitiveComponent Object Reference") (OtherActor :type "Actor Object Reference") (OtherComp :type "PrimitiveComponent Object Reference") (OtherBodyIndex :type Integer) (bFromSweep :type Boolean) (SweepResult :type "HitResult Structure (by ref)"))
  (bind _asbp_wall (cast `/Game/Blueprints/Buildings/Wall/BP_Wall` OtherActor))
  (set `self.WallToAttack` _asbp_wall)
  (set `self.IsAttacking` true)
  (`MovementComponent.StopMovementImmediately` (`self.CharacterMovement`))
  (`PrimitiveComponent.SetSimulatePhysics` (`self.CapsuleComponent`) true))

(event `self.WallDetector.OnComponentEndOverlap`
  (params (OverlappedComponent :type "PrimitiveComponent Object Reference") (OtherActor :type "Actor Object Reference") (OtherComp :type "PrimitiveComponent Object Reference") (OtherBodyIndex :type Integer))
  (set `self.IsAttacking` false)
  (`MovementComponent.StopMovementImmediately` (`self.CharacterMovement`))
  (`KismetSystemLibrary.Delay` 2.0)
  (`PrimitiveComponent.SetSimulatePhysics` (`self.CapsuleComponent`) false))

(event `MoveToHQ`
  (bind (_returnvalue_x _returnvalue_y _returnvalue_z) (`KismetMathLibrary.BreakVector` (`self.K2_GetActorLocation`)))
  (bind _isalive (`self.IsAlive`))
  (bind _returnvalue_x_2 (`KismetMathLibrary.BreakVector` (`self.K2_GetActorLocation` (`CTGameModeLevel.GetBuildingHQ` (`self.GetGameMode`)))))
  (if (and (not (`self.IsAttacking`)) _isalive)
    (`|AIMoveTo` self (`KismetMathLibrary.MakeVector` _returnvalue_x_2 _returnvalue_y _returnvalue_z) null 0.0)
    (elif (not _isalive)
      (`MovementComponent.StopMovementImmediately` (`self.CharacterMovement`)))))

(event `Attack`
  (bind _walltoattack (`self.WallToAttack`))
  (bind _returnvalue_x (`KismetMathLibrary.BreakVector` (`KismetMathLibrary.Normal` (- (`self.K2_GetActorLocation` (`CTGameModeLevel.GetBuildingHQ` (`self.GetGameMode`))) (`self.K2_GetActorLocation`)))))
  (`KismetSystemLibrary.Delay` 2.0)
  (if (`self.IsAttacking`)
    (`PaperZDAnimInstance.JumpToNode` (`self.GetAnimInstance`) "JumpAttack" "Locomotion")
    (`KismetSystemLibrary.Delay` 0.5)
    (`PrimitiveComponent.AddImpulse` (`self.CapsuleComponent`) (* (+ (`KismetMathLibrary.MakeVector` (`KismetMathLibrary.Conv_IntToDouble` (`KismetMathLibrary.RandomIntegerInRange` 1800 2000)) 0.0 50.0) (* (0.0 0.0 1.0) 300.0)) _returnvalue_x) "None" true)
    (`KismetSystemLibrary.Delay` 0.2)
    (`/Engine/EditorBlueprintResources/StandardMacros.IsValid` _walltoattack
      (:`Is Valid`
        (`/Game/Blueprints/Buildings/Wall/BP_Wall.AddDamage` _walltoattack (`self.Damage`))
        (set `self.WallToAttack` null)))))

(fn `AddDamage`
  (params (Damage :type "Float (double-precision)"))
  (locals (OldValue :type "Float (double-precision)" :default 0.0))
  (bind _currenthitpoints (`self.CurrentHitpoints`))
  (set `local.OldValue` _currenthitpoints)
  (bind _output_get (set `self.CurrentHitpoints` (- _currenthitpoints (`local.Damage`))))
  (`self.CurrentHitpointsChanged` (`local.OldValue`) _output_get)
  (if (<= (`self.CurrentHitpoints`) 0.0)
    (set `self.CurrentHitpoints` 0.0)
    (`self.CurrentHitpointsDepleted`)
    (else
      (`PaperZDAnimInstance.JumpToNode` (`self.GetAnimInstance`) "JumpHit" "Locomotion"))))

(fn `GetDamage`
  (returns (Damage :type "Float (double-precision)"))
  (return (`self.Damage`)))

(fn `IsAlive`
  (returns (IsAlive :type Boolean))
  (return (> (`self.CurrentHitpoints`) 0.0)))

(fn `IsArcherTarget`
  (returns (Target :type "CTEnemyNPCCharacter Object Reference"))
  (return self))

(fn `OnCurrentHitpointsDepleted`
  (`self.K2_DestroyActor`))

(fn `UserConstructionScript`)