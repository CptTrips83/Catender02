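; Friendly NPC archer that runs the BT_Archer behavior tree, shoots nearby targets and gathers pickups for the player.
; A shooting sphere maintains the target list; Tick launches a projectile at the first entry, throttled by a randomized cooldown timer.
; Its pickup collision stores looted resources and relaunches them as Gold or Meat when the player overlaps, with start/end events pausing looting meanwhile.
; It also supplies random X-axis patrol points within a box.
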(event `self.ReceiveBeginPlay`
  (`|ExecutionSequence`
    (:`then_0`
      (bind _asaic_friendly_npc (cast `/Game/AI/FriendlyNPC/AIC_FriendlyNPC` (`self.GetController`)))
      (`/Game/AI/FriendlyNPC/AIC_FriendlyNPC.SetBehavior` _asaic_friendly_npc "/Game/AI/FriendlyNPC/Archer/BT_Archer.BT_Archer"))
    (:`then_1`
      (`self.BindPickupEvents`))))

(event `self.ReceiveTick`
  (params (DeltaSeconds :type "Float (single-precision)"))
  (if (not (`self.IsShooting`))
    (`self.ShootProjectile`)))

(event `self.ShootingSphere.OnComponentBeginOverlap`
  (params (OverlappedComponent :type "PrimitiveComponent Object Reference") (OtherActor :type "Actor Object Reference") (OtherComp :type "PrimitiveComponent Object Reference") (OtherBodyIndex :type Integer) (bFromSweep :type Boolean) (SweepResult :type "HitResult Structure (by ref)"))
  (bind _target (message `/Game/Blueprints/Interfaces/Archer/BPINT_ArcherTarget.IsArcherTarget` OtherActor))
  (`/Engine/EditorBlueprintResources/StandardMacros.IsValid` _target
    (:`Is Valid`
      (`KismetArrayLibrary.Array_AddUnique` (`self.Targets`) _target))))

(event `self.ShootingSphere.OnComponentEndOverlap`
  (params (OverlappedComponent :type "PrimitiveComponent Object Reference") (OtherActor :type "Actor Object Reference") (OtherComp :type "PrimitiveComponent Object Reference") (OtherBodyIndex :type Integer))
  (bind _target (message `/Game/Blueprints/Interfaces/Archer/BPINT_ArcherTarget.IsArcherTarget` OtherActor))
  (`/Engine/EditorBlueprintResources/StandardMacros.IsValid` _target
    (:`Is Valid`
      (`KismetArrayLibrary.Array_RemoveItem` (`self.Targets`) _target)
      (`self.ResetShooting`))))

(event `self.ArcherPickupCollision.OnComponentBeginOverlap`
  (params (OverlappedComponent :type "PrimitiveComponent Object Reference") (OtherActor :type "Actor Object Reference") (OtherComp :type "PrimitiveComponent Object Reference") (OtherBodyIndex :type Integer) (bFromSweep :type Boolean) (SweepResult :type "HitResult Structure (by ref)"))
  (`self.ProcessPickupInteraction` OtherActor))

(event `DropPickups`
  (if (not (`self.IsDropping`))
    (`self.OnDropPickupsStarted`)
    (`/Engine/EditorBlueprintResources/StandardMacros.DoOnce` false :!label _label
      (:`Completed`
        (for _array_element (`self.Pickups`)
          (`self.SpawnPickup` _array_element))
        (`self.OnDropPickupsEnded`)
        (goto _label :!via `Reset`)))))

(event `DropPickupsEnded`
  (`KismetArrayLibrary.Array_Clear` (`self.Pickups`))
  (`KismetSystemLibrary.Delay` 2.0)
  (set `self.IsDropping` false))

(fn `BindPickupEvents`
  (add `self.OnDropPickupsStarted` (`|CreateDelegate` :!event `DropPickupsStarted`))
  (add `self.OnDropPickupsEnded` (`|CreateDelegate` :!event `DropPickupsEnded`)))

(fn `CreateProjectile`
  (params (Target :type "CTEnemyNPCCharacter Object Reference"))
  (returns (Projectile :type "/Game/Blueprints/Projectiles/BP_Projectile_BASE Object Reference"))
  (bind _returnvalue (`|SpawnActorFromClass` "/Game/Blueprints/Projectiles/BP_Projectile_BASE.BP_Projectile_BASE_C" (`KismetMathLibrary.MakeTransform` (`SceneComponent.K2_GetComponentLocation` (`self.Scene`))) "Undefined" "MultiplyWithRoot" null null))
  (`/Engine/EditorBlueprintResources/StandardMacros.IsValid` _returnvalue
    (:`Is Valid`
      (`CTProjectile.LaunchProjectile` _returnvalue (`self.K2_GetActorLocation` (`local.Target`)) 150.0 0.2)
      (`self.PlayShootingSound`)
      (return null))))

(fn `DropPickupsStarted`
  (set `self.IsDropping` true))

(fn `GetNextPatrolLocation`
  (returns (Location :type "Vector Structure"))
  (bind (_returnvalue_x _returnvalue_y _returnvalue_z) (`KismetMathLibrary.BreakVector` (`self.K2_GetActorLocation`)))
  (return (`KismetMathLibrary.MakeVector` (`self.GetRandomPositionInBox` (`self.PatrolBox`)) _returnvalue_y _returnvalue_z)))

(fn `GetNextTarget`
  (returns (Target :type "CTEnemyNPCCharacter Object Reference"))
  (if (> (`KismetArrayLibrary.Array_Length` (`self.Targets`)) 0)
    (return (`|GetArrayItem` (`self.Targets`)))
    (else
      (return null))))

(fn `GetShootingCooldown`
  (returns (ShootinCooldown :type "Float (double-precision)"))
  (return (`KismetMathLibrary.RandomFloatInRange` (`self.MinShootingCooldown`) (`self.MaxShootingCooldown`))))

(fn `LootPickup`
  (params (Pickup :type "/Game/Blueprints/Pickups/BP_Pickup_BASE Object Reference"))
  (if (not (`self.IsDropping`))
    (for _array_element (`CTPickable.Resources` Pickup)
      (`KismetArrayLibrary.Array_Add` (`self.Pickups`) _array_element))
    (`self.K2_DestroyActor` Pickup)))

(fn `PlayShootingSound`
  (`GameplayStatics.PlaySoundAtLocation` "/Game/SFX/Archer/Releasing_string__Bow__1_Cue.Releasing_string__Bow__1_Cue" (`self.K2_GetActorLocation`) (struct) 1.0 1.0 0.0 null null null null))

(fn `ProcessPickupInteraction`
  (params (`Other Actor` :type "Actor Object Reference"))
  (`|ExecutionSequence`
    (:`then_0`
      (bind _asbp_pickup_base (cast `/Game/Blueprints/Pickups/BP_Pickup_BASE` (`local.Other Actor`)))
      (`self.LootPickup` _asbp_pickup_base))
    (:`then_1`
      (cast `/Game/Blueprints/Character/Player/BP_PlayerCharacter` (`local.Other Actor`))
      (`self.DropPickups`))))

(fn `ResetShooting`
  (set `self.IsShooting` false)
  (`KismetSystemLibrary.K2_ClearAndInvalidateTimerHandle` (`self.ShootingTimer`)))

(fn `ShootProjectile`
  (locals (NextTarget :type "CTEnemyNPCCharacter Object Reference"))
  (bind _target (`self.GetNextTarget`))
  (`/Engine/EditorBlueprintResources/StandardMacros.IsValid` _target
    (:`Is Valid`
      (set `local.NextTarget` _target)
      (set `self.IsShooting` true)
      (`self.CreateProjectile` _target)
      (bind _returnvalue (`KismetSystemLibrary.K2_SetTimerDelegate` (`|CreateDelegate` :!event `ResetShooting`) (`self.GetShootingCooldown`)))
      (set `self.ShootingTimer` _returnvalue))))

(fn `SpawnPickup`
  (params (Pickup :type "Resource Structure"))
  (bind (_returnvalue_x _returnvalue_y _returnvalue_z) (`KismetMathLibrary.BreakVector` (`SceneComponent.K2_GetComponentLocation` (`self.ScenePickups`))))
  (bind _returnvalue (`|SpawnActorFromClass` (select `EResourceType` Pickup_ResourceType :`Gold` "/Game/Blueprints/Pickups/BP_Gold.BP_Gold_C" :`Meat` "/Game/Blueprints/Pickups/BP_Meat.BP_Meat_C" :!type "Actor Class Reference") (`KismetMathLibrary.MakeTransform` (`KismetMathLibrary.MakeVector` (+ (`KismetMathLibrary.RandomFloatInRange` -5.0 5.0) _returnvalue_x) _returnvalue_y _returnvalue_z)) "AlwaysSpawn" "MultiplyWithRoot" null null))
  (bind _asbp_pickup_base (cast `/Game/Blueprints/Pickups/BP_Pickup_BASE` _returnvalue))
  (`/Game/Blueprints/Pickups/BP_Pickup_BASE.LaunchPickup` _asbp_pickup_base))

(fn `UserConstructionScript`
  (`parent.UserConstructionScript`))