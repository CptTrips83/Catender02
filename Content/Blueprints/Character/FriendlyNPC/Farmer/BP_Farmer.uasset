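; Farmer NPC that extends its parent's working behavior with timed movement, animation and sound.
; ProcessWorking accumulates progress by delta time toward a random threshold, which is rolled only at BeginPlay.
; While working past that threshold, it requests a move to a random X within its assigned buildable's construction box, only by day, keeping Y and Z.
; After a short delay, it jumps the locomotion state machine to work and plays a purr.
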(event `self.ReceiveBeginPlay`
  (`parent.ReceiveBeginPlay`)
  (`self.ResetWorkingProgress`))

(event `self.ProcessWorking`
  (`parent.ProcessWorking`)
  (`|ExecutionSequence`
    (:`then_0`
      (set `self.CurrentWorkingProgress` (+ (`self.CurrentWorkingProgress`) (* (`self.WorkingProgressValue`) (`GameplayStatics.GetWorldDeltaSeconds`)))))
    (:`then_1`
      (if (`self.HasWorkingProgress`)
        (`self.MoveToRandomPosition`)
        (`KismetSystemLibrary.Delay` 0.5)
        (`self.PlayWorkAnimation`)
        (`self.PlayWorkSound`)))))

(event `MoveToRandomPosition`
  (bind (_returnvalue_x _returnvalue_y _returnvalue_z) (`KismetMathLibrary.BreakVector` (`self.K2_GetActorLocation`)))
  (if (`self.CanWork`)
    (`|AIMoveTo` self (`KismetMathLibrary.MakeVector` (`self.GetRandomPositionInBox` (`CTBuildable.ConstructionSiteBoxComponent` (`self.GetAssignedBuildable`))) _returnvalue_y _returnvalue_z) null 0.0)))

(fn `CanWork`
  (returns (CanWork :type Boolean))
  (return (and (`CTWorldDayTimeComponent.IsDay` (`CTGameModeLevel.WorldDayTimeComponent` (`self.GetGameMode`))) (`KismetSystemLibrary.IsValid` (`self.GetAssignedBuildable`)))))

(fn `HasWorkingProgress`
  (returns (HasProgress :type Boolean))
  (return (and (>= (`self.CurrentWorkingProgress`) (`self.NeededWorkingProgress`)) (`self.GetIsWorking`))))

(fn `PlayWorkAnimation`
  (`PaperZDAnimInstance.JumpToNode` (`self.GetAnimInstance`) "JumpWork" "Locomotion"))

(fn `PlayWorkSound`
  (`GameplayStatics.PlaySoundAtLocation` "/Game/SFX/Farmer/FarmerPurr_Cue.FarmerPurr_Cue" (`self.K2_GetActorLocation`) (struct) 1.0 1.0 0.0 null null null null))

(fn `ResetWorkingProgress`
  (set `self.CurrentWorkingProgress` 0.0)
  (set `self.NeededWorkingProgress` (`KismetMathLibrary.RandomFloatInRange` (`self.MinNeededWorkinProgress`) (`self.MaxNeededWorkingProgress`))))

(fn `UserConstructionScript`
  (`parent.UserConstructionScript`))