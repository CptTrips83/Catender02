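; BP_Kitten is a friendly NPC kitten that can be recruited and can look up a workshop.
; Recruit sets the IsRecruited flag and GetRecruited returns it.
; GetNearestWorkingSite returns the first BP_Workshop_BASE actor whose HasTool is true, or nothing if none qualifies, without comparing distances despite its name.
; The event graph holds only disabled placeholder events, so the Blueprint drives no behavior itself.
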(fn `GetNearestWorkingSite`
  (returns (ReturnValue :type "CTBuildable Object Reference"))
  (bind _outactors (`GameplayStatics.GetAllActorsOfClass` "/Game/Blueprints/Buildings/Workshop/BP_Workshop_BASE.BP_Workshop_BASE_C"))
  (for _array_element _outactors
    (if (`/Game/Blueprints/Buildings/Workshop/BP_Workshop_BASE.HasTool` _array_element)
      (return _array_element)))
  (return null))

(fn `GetRecruited`
  (returns (IsRecruited :type Boolean))
  (return (`self.IsRecruited`)))

(fn `Recruit`
  (set `self.IsRecruited` true))

(fn `UserConstructionScript`
  (`parent.UserConstructionScript`))