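; BP_Worker is a friendly NPC that builds the buildable assigned to it as a construction site.
; Each ProcessWorking call waits a random interval, adds progress to the buildable's BuildingComponent and jumps the Locomotion state machine to the work animation.
; It then AI-moves to a random X within the site's box, keeping its own Y and Z.
; A change to working state plays a meow sound.
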(event `self.ReceiveBeginPlay`
  (`parent.ReceiveBeginPlay`)
  (add `self.OnWorkingIsChanged` (`|CreateDelegate` :!event `Is Working Changed`)))

(event `WorkOnConstructionSite`
  (bind _constructionsite (`self.GetConstructionSite`))
  (bind _returnvalue (`self.GetAssignedBuildable`))
  (bind (_returnvalue_x _returnvalue_y _returnvalue_z) (`KismetMathLibrary.BreakVector` (`self.K2_GetActorLocation`)))
  (if (`self.GetIsWorking`)
    (`/Engine/EditorBlueprintResources/StandardMacros.IsValid` _returnvalue
      (:`Is Valid`
        (`KismetSystemLibrary.Delay` (`self.GetConstructionProgressInterval`))
        (`/Engine/EditorBlueprintResources/StandardMacros.IsValid` _returnvalue
          (:`Is Valid`
            (`CTBuildingComponent.AddProgressToBuilding` (`CTBuildable.BuildingComponent` _returnvalue) (`self.ConstructionProgress`))
            (`self.PlayWorkAnimation`)
            (`/Engine/EditorBlueprintResources/StandardMacros.IsValid` _constructionsite
              (:`Is Valid`
                (`|AIMoveTo` self (`KismetMathLibrary.MakeVector` (`self.GetRandomPositionInBox` (`CTBuildable.ConstructionSiteBoxComponent` _constructionsite)) _returnvalue_y _returnvalue_z) null 0.0)))))))))

(event `self.StartWorking`
  (`parent.StartWorking`))

(event `self.ProcessWorking`
  (`parent.ProcessWorking`)
  (`self.WorkOnConstructionSite`))

(event `self.StopWorking`
  (`parent.StopWorking`))

(fn `Get Nearest Construction Site`
  (returns (Buildable :type "CTBuildable Object Reference"))
  (return (`self.GetNearestWorkingSite`)))

(fn `GetConstructionProgressInterval`
  (returns (Interval :type "Float (double-precision)"))
  (return (`KismetMathLibrary.RandomFloatInRange` (`self.MinConstructionProgressInterval`) (`self.MaxConstructionProgressInterval`))))

(fn `GetConstructionSite`
  (returns (ConstructionSite :type "CTBuildable Object Reference"))
  (return (`self.GetAssignedBuildable`)))

(fn `Is Working Changed`
  (params (NPC :type "CTFriendlyNPCCharacter Object Reference") (`Old Value` :type Boolean) (`New Value` :type Boolean))
  (if `New Value`
    (`GameplayStatics.PlaySoundAtLocation` "/Game/SFX/Worker/Miau_2.Miau_2" (`self.K2_GetActorLocation`) (struct) 1.0 1.0 0.0 null null null null)))

(fn `PlayWorkAnimation`
  (`PaperZDAnimInstance.JumpToNode` (`self.GetAnimInstance`) "JumpWork" "Locomotion"))

(fn `UserConstructionScript`)