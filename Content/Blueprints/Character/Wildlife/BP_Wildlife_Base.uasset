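; Base wildlife actor for cat levels that roams under AI control, can be targeted by archers, and drops loot when destroyed.
; On BeginPlay it gives its AIC_FriendlyNPC controller the BT_Wildlife behavior tree and registers with GM_CatLevel's WorldWildlifeComponent.
; InflictDamage destroys it immediately; Destroyed then unregisters it and randomly spawns either BP_Gold or BP_Meat at its location.
; IsArcherTarget returns the actor itself.
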(event `self.ReceiveBeginPlay`
  (`|ExecutionSequence`
    (:`then_0`
      (bind _asaic_friendly_npc (cast `/Game/AI/FriendlyNPC/AIC_FriendlyNPC` (`self.GetController`)))
      (`/Game/AI/FriendlyNPC/AIC_FriendlyNPC.SetBehavior` _asaic_friendly_npc "/Game/AI/FriendlyNPC/Wildlife/BT_Wildlife.BT_Wildlife"))
    (:`then_1`
      (bind _asgm_cat_level (cast `/Game/Blueprints/GameModes/GM_CatLevel` (`GameplayStatics.GetGameMode`)))
      (`CTWorldWildlifeComponent.AddWildlife` (`CTGameModeLevel.WorldWildlifeComponent` _asgm_cat_level) self))))

(event `self.ReceiveDestroyed`
  (bind _asgm_cat_level (cast `/Game/Blueprints/GameModes/GM_CatLevel` (`GameplayStatics.GetGameMode`)))
  (`CTWorldWildlifeComponent.RemoveWildlife` (`CTGameModeLevel.WorldWildlifeComponent` _asgm_cat_level) self)
  (`self.SpawnLoot`))

(event `/Game/Blueprints/Interfaces/Archer/BPINT_Damage.InflictDamage`
  (params (Damage :type "Float (double-precision)"))
  (`self.K2_DestroyActor`))

(fn `IsArcherTarget`
  (returns (Target :type "CTEnemyNPCCharacter Object Reference"))
  (return self))

(fn `SpawnLoot`
  (if (`KismetMathLibrary.RandomBool`)
    (`|SpawnActorFromClass` "/Game/Blueprints/Pickups/BP_Gold.BP_Gold_C" (`KismetMathLibrary.MakeTransform` (`self.K2_GetActorLocation`)) "AlwaysSpawn" "MultiplyWithRoot" null null)
    (else
      (`|SpawnActorFromClass` "/Game/Blueprints/Pickups/BP_Meat.BP_Meat_C" (`KismetMathLibrary.MakeTransform` (`self.K2_GetActorLocation`)) "AlwaysSpawn" "MultiplyWithRoot" null null))))

(fn `UserConstructionScript`)