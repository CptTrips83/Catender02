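; BP_Turtle is a turtle wildlife Blueprint that puts its animation to sleep when night falls.
; On BeginPlay it binds to the day-changed event of the WorldDayTimeComponent on GM_CatLevel.
; OnNightTime reacts only to day-to-night transitions, jumping the anim instance's Locomotion state machine to the JumpSleep node.
; It has no branch for the return to day.
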(event `self.ReceiveBeginPlay`
  (`parent.ReceiveBeginPlay`)
  (bind _asgm_cat_level (cast `/Game/Blueprints/GameModes/GM_CatLevel` (`GameplayStatics.GetGameMode`)))
  (add `CTWorldDayTimeComponent.OnDayChanged` (`CTGameModeLevel.WorldDayTimeComponent` _asgm_cat_level) (`|CreateDelegate` :!event `OnNightTime`)))

(fn `OnNightTime`
  (params (OldValue :type Integer) (NewValue :type Integer) (OldIsDay :type Boolean) (NewIsDay :type Boolean))
  (if (!= OldIsDay NewIsDay)
    (if (not (`local.NewIsDay`))
      (`PaperZDAnimInstance.JumpToNode` (`self.GetAnimInstance`) "JumpSleep" "Locomotion"))))

(fn `UserConstructionScript`
  (`parent.UserConstructionScript`))