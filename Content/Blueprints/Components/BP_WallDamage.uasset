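; BP_WallDamage is a component that gives an owning BP_Wall visual damage stages as it takes damage.
; While the wall is active, each damage change is converted to a fraction of hit points and checked against threshold keys for the current building level.
; Each newly crossed threshold broadcasts a damage-info change with its flipbook.
; The change handler swaps the wall's flipbook and spawns random debris actors around it.
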(event `self.ReceiveBeginPlay`
  (bind _asbp_wall (cast `/Game/Blueprints/Buildings/Wall/BP_Wall` (`self.GetOwner`)))
  (bind _output_get (set `self.Owning Wall` _asbp_wall))
  (add `/Game/Blueprints/Buildings/Wall/BP_Wall.OnDamageChanged` _output_get (delegate `DamageChanged`))
  (add `self.OnWallDamageInfoChange` (`|CreateDelegate` :!event `WallDamageInfoChanged`)))

(event `DamageChanged`
  (params (Target :type "/Game/Blueprints/Buildings/Wall/BP_Wall Object Reference") (OldDamage :type "Float (double-precision)") (NewDamage :type "Float (double-precision)"))
  (if (`self.IsWallActive`)
    (`self.UpdateWall` OldDamage NewDamage)))

(fn `CalcDamagePercentage`
  (params (Damage :type "Float (double-precision)") (HitPoints :type "Float (double-precision)"))
  (returns (Percentage :type "Float (double-precision)"))
  (if (!= HitPoints 0.0)
    (return (/ (`local.Damage`) (`local.HitPoints`)))
    (else
      (return 0.0))))

(fn `FireDebris`
  (for _ (range (+ (`KismetMathLibrary.RandomIntegerInRange` 3 8) 1))
    (`|SpawnActorFromClass` (`KismetArrayLibrary.Array_Random` (`self.DebrisClasses`)) (`KismetMathLibrary.MakeTransform` (+ (`Actor.K2_GetActorLocation` (`self.Owning Wall`)) (`KismetMathLibrary.MakeVector` (`KismetMathLibrary.RandomFloatInRange` -5.0 5.0) 0.0 (`KismetMathLibrary.RandomFloatInRange` -5.0 5.0)))) "AlwaysSpawn" "MultiplyWithRoot" null null)))

(fn `GetWallDamageInfo`
  (params (CurrentLevel :type Integer))
  (returns (WallDamageInfo :type "/Game/Blueprints/Structures/S_WallDamageInfo Structure"))
  (return (`BlueprintMapLibrary.Map_Find` (`self.WallDamageInfos`) CurrentLevel)))

(fn `IsWallActive`
  (returns (ReturnValue :type Boolean))
  (return (`|EnumEquality` (`CTBuildingComponent.GetBuildingState` (`CTBuildable.BuildingComponent` (`self.Owning Wall`))) "Active")))

(fn `UpdateWall`
  (params (OldDamage :type "Float (double-precision)") (NewDamage :type "Float (double-precision)"))
  (locals (OldDamagePercentage :type "Float (double-precision)") (NewDamagePercentage :type "Float (double-precision)"))
  (bind _newdamagepercentage (`local.NewDamagePercentage`))
  (bind _walldamageinfo_damagedsprites (break `/Game/Blueprints/Structures/S_WallDamageInfo` (`self.GetWallDamageInfo` (`CTBuildingComponent.GetCurrentBuildingLevel` (`CTBuildable.BuildingComponent` (`self.Owning Wall`))))))
  (`|ExecutionSequence`
    (:`then_0`
      (set `local.OldDamagePercentage` (`self.CalcDamagePercentage` (`local.OldDamage`) (`/Game/Blueprints/Buildings/Wall/BP_Wall.GetHitPoints` (`self.Owning Wall`))))
      (set `local.NewDamagePercentage` (`self.CalcDamagePercentage` (`local.NewDamage`) (`/Game/Blueprints/Buildings/Wall/BP_Wall.GetHitPoints` (`self.Owning Wall`)))))
    (:`then_1`
      (bind _keys (`BlueprintMapLibrary.Map_Keys` _walldamageinfo_damagedsprites))
      (for _array_element _keys
        (if (and (> _array_element (`local.OldDamagePercentage`)) (<= _array_element _newdamagepercentage))
          (`self.OnWallDamageInfoChange` (`BlueprintMapLibrary.Map_Find` _walldamageinfo_damagedsprites _array_element) _newdamagepercentage))))))

(fn `UpdateWallSprite`
  (params (Sprite :type "PaperFlipbook Object Reference"))
  (`PaperFlipbookComponent.SetFlipbook` (`PaperCharacter.Sprite` (`self.Owning Wall`)) Sprite))

(fn `WallDamageInfoChanged`
  (params (Sprite :type "PaperFlipbook Object Reference") (DamagePercentage :type "Float (double-precision)"))
  (`self.UpdateWallSprite` Sprite)
  (`self.FireDebris`))