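; World archer manager that spreads cat archers between defensive walls on the left and right of the HQ.
; At BeginPlay it binds to existing walls' building-state changes and archer workshops' spawn events, tracking new archers in a list.
; Each update alternates archers' home building via FlipFlop between each side's first active, non-critically-damaged wall in descending sort order, falling back to the HQ.
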(event `self.ReceiveBeginPlay`
  (`|ExecutionSequence`
    (:`then_0`
      (bind _asgm_cat_level (cast `/Game/Blueprints/GameModes/GM_CatLevel` (`GameplayStatics.GetGameMode`)))
      (set `self.Owning Gamemode` _asgm_cat_level))
    (:`then_1`
      (`self.BindEvents`))))

(fn `AddArcher`
  (params (Archer :type "/Game/Blueprints/Character/FriendlyNPC/Archer/BP_Archer Object Reference"))
  (`KismetArrayLibrary.Array_Add` (`self.Archers`) Archer))

(fn `BindEvents`
  (`|ExecutionSequence`
    (:`then_0`
      (bind _towers (`self.GetAllDefenseInWorld`))
      (for _array_element _towers
        (add `CTBuildingComponent.OnBuildingStateChanged` (`CTBuildable.BuildingComponent` _array_element) (`|CreateDelegate` :!event `TowerBuildingStateChanged`))))
    (:`then_1`
      (bind _outactors (`GameplayStatics.GetAllActorsOfClass` "/Game/Blueprints/Buildings/Workshop/BP_Workshop_Archer.BP_Workshop_Archer_C"))
      (for _array_element_2 _outactors
        (add `/Game/Blueprints/Buildings/Workshop/BP_Workshop_BASE.NewCatSpawned` _array_element_2 (`|CreateDelegate` :!event `OnNewArcherSpawned`))))))

(fn `GetActiveTowerInWorld`
  (returns (LeftTower :type "CTBuilding Object Reference") (RightTower :type "CTBuilding Object Reference"))
  (locals (FoundLeftTower :type "CTBuilding Object Reference") (FoundRightTower :type "CTBuilding Object Reference"))
  (bind _owning_gamemode (`self.Owning Gamemode`))
  (bind _owning_gamemode_2 (`self.Owning Gamemode`))
  (`|ExecutionSequence`
    (:`then_0`
      (for _array_element (`CTWorldBuildableComponent.GetBuildablesByDirection` (`CTGameModeLevel.WorldBuildableComponent` _owning_gamemode) (`CTGameModeLevel.GetBuildingHQ` _owning_gamemode) "Left" false)
        (bind _asbp_wall (cast `/Game/Blueprints/Buildings/Wall/BP_Wall` _array_element))
        (if (and (not (`/Game/Blueprints/Buildings/Wall/BP_Wall.IsCriticalDamaged` _asbp_wall)) (`|EnumEquality` (`CTBuildingComponent.GetBuildingState` (`CTBuildable.BuildingComponent` _asbp_wall)) "Active"))
          (set `local.FoundLeftTower` _asbp_wall)
          (break))))
    (:`then_1`
      (for _array_element_2 (`CTWorldBuildableComponent.GetBuildablesByDirection` (`CTGameModeLevel.WorldBuildableComponent` _owning_gamemode_2) (`CTGameModeLevel.GetBuildingHQ` _owning_gamemode_2) "Right" false)
        (bind _asbp_wall_2 (cast `/Game/Blueprints/Buildings/Wall/BP_Wall` _array_element_2))
        (if (and (not (`/Game/Blueprints/Buildings/Wall/BP_Wall.IsCriticalDamaged` _asbp_wall_2)) (`|EnumEquality` (`CTBuildingComponent.GetBuildingState` (`CTBuildable.BuildingComponent` _asbp_wall_2)) "Active"))
          (set `local.FoundRightTower` _asbp_wall_2)
          (break))))
    (:`then_2`
      (`local.FoundLeftTower`
        (:`then`)
        (:`else`
          (set `local.FoundLeftTower` (`CTGameModeLevel.GetBuildingHQ` (`self.Owning Gamemode`))))))
    (:`then_3`
      (`local.FoundRightTower`
        (:`then`)
        (:`else`
          (set `local.FoundRightTower` (`CTGameModeLevel.GetBuildingHQ` (`self.Owning Gamemode`))))))
    (:`then_4`
      (return (`local.FoundLeftTower`) (`local.FoundRightTower`)))))

(fn `GetAllDefenseInWorld`
  (returns (Towers :type "Array of /Game/Blueprints/Buildings/Wall/BP_Wall Object Reference"))
  (locals (Result :type "Array of /Game/Blueprints/Buildings/Wall/BP_Wall Object Reference"))
  (for _array_element (`CTWorldBuildableComponent.GetBuildables` (`CTGameModeLevel.WorldBuildableComponent` (`self.Owning Gamemode`)))
    (bind _asbp_wall (cast `/Game/Blueprints/Buildings/Wall/BP_Wall` _array_element))
    (`KismetArrayLibrary.Array_Add` (`local.Result`) _asbp_wall))
  (return (`local.Result`)))

(fn `OnNewArcherSpawned`
  (params (NewCat :type "CTFriendlyNPCCharacter Object Reference"))
  (bind _asbp_archer (cast `/Game/Blueprints/Character/FriendlyNPC/Archer/BP_Archer` NewCat))
  (`self.AddArcher` _asbp_archer)
  (`self.TowerBuildingStateChanged` (`CTGameModeLevel.GetBuildingHQ` (`self.Owning Gamemode`))))

(fn `RemoveArcher`
  (params (Archer :type "/Game/Blueprints/Character/FriendlyNPC/Archer/BP_Archer Object Reference"))
  (`KismetArrayLibrary.Array_RemoveItem` (`self.Archers`) Archer))

(fn `TowerBuildingStateChanged`
  (params (Buildable :type "CTBuildable Object Reference") (OldState :type "EBuildingState Enum" :default "Invisible") (NewState :type "EBuildingState Enum" :default "Invisible"))
  (for _array_element (`self.Archers`)
    (`/Engine/EditorBlueprintResources/StandardMacros.FlipFlop`
      (:`A`
        (`CTFriendlyNPCCharacter.SetHomeBuilding` _array_element (`self.GetActiveTowerInWorld`)))
      (:`B`
        (`CTFriendlyNPCCharacter.SetHomeBuilding` _array_element (`.RightTower` (`self.GetActiveTowerInWorld`)))))))