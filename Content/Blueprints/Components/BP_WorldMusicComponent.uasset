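; BP_WorldMusicComponent is a component that keeps world music playing and restarts playback as the current track nears its end.
; On BeginPlay it caches GI_Catender, sends a play request with its Music and fade times, and binds to the game instance's playback percentage updates.
; When playback reaches a configurable percentage threshold, it sends the same request again with crossfade times.
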(event `self.ReceiveBeginPlay`
  (bind _asgi_catender (cast `/Game/Blueprints/GameInstance/GI_Catender` (`GameplayStatics.GetGameInstance`)))
  (set `self.Game Instance` _asgi_catender)
  (`self.PlayNewTrack`)
  (add `/Game/Blueprints/GameInstance/GI_Catender.PlaybackPercentageChanged` (`self.Game Instance`) (`|CreateDelegate` :!event `OnPlaybackPercentageChanged`)))

(fn `OnPlaybackPercentageChanged`
  (params (`Game Instance` :type "/Game/Blueprints/GameInstance/GI_Catender Object Reference") (`Playback Percent` :type "Float (double-precision)"))
  (if (>= `Playback Percent` (`self.ChangeMusicOnPlaybackPercentage`))
    (`self.PlayNewTrack`)))

(fn `PlayNewTrack`
  (message `/Game/Blueprints/Interfaces/GameInstance/BPINT_MusicPlayer.PlayMusic` (`self.Game Instance`) (`self.Music`) (`self.FadeOutTimeOld`) (`self.FadeInTimeNew`)))