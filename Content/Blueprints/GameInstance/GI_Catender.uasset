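; Game instance for Catender that manages background music, keeping it playing across level transitions.
; PlayMusic fades out any active track through StopMusic, then creates a persistent 2D audio component and fades the new one in.
; Pause and resume act on the active player, whose playback percent is rebroadcast through the PlaybackPercentageChanged dispatcher for other objects to follow.
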(event `/Game/Blueprints/Interfaces/GameInstance/BPINT_MusicPlayer.PlayMusic`
  (params (Music :type "SoundBase Object Reference") (FadeOutTimeOld :type "Float (double-precision)") (FadeInTimeNew :type "Float (double-precision)"))
  (bind _activemusicplayer (`self.ActiveMusicPlayer`))
  (set `self.Music` Music)
  (set `self.Fade Out Time Old` FadeOutTimeOld)
  (set `self.Fade in Time New` FadeInTimeNew)
  (`/Engine/EditorBlueprintResources/StandardMacros.IsValid` (`self.ActiveMusicPlayer`)
    (:`Is Valid`
      (`self.StopMusic` (`self.Fade Out Time Old`)))
    (:`Is Not Valid`
      _))
  (bind _returnvalue (`GameplayStatics.CreateSound2D` (`self.Music`) 1.0 1.0 0.0 null true))
  (bind _output_get (set `self.ActiveMusicPlayer` _returnvalue))
  (`AudioComponent.FadeIn` _output_get (`self.Fade in Time New`) 1.0 0.0 "Linear")
  (add `AudioComponent.OnAudioPlaybackPercent` _activemusicplayer (`|CreateDelegate` :!event `OnPlaybackPercentageChanged`))
  (`AudioComponent.Play` _activemusicplayer 0.0))

(event `/Game/Blueprints/Interfaces/GameInstance/BPINT_MusicPlayer.StopMusic`
  (params (FadeOutTime :type "Float (double-precision)"))
  (bind _output_get (set `self.FadeoutMusicPlayer` (`self.ActiveMusicPlayer`)))
  (`AudioComponent.FadeOut` _output_get FadeOutTime 0.0 "Linear")
  (clear `AudioComponent.OnAudioPlaybackPercent` (`self.ActiveMusicPlayer`)))

(event `/Game/Blueprints/Interfaces/GameInstance/BPINT_MusicPlayer.PauseMusic`
  (`AudioComponent.SetPaused` (`self.ActiveMusicPlayer`) true))

(event `/Game/Blueprints/Interfaces/GameInstance/BPINT_MusicPlayer.ResumeMusic`
  (`AudioComponent.SetPaused` (`self.ActiveMusicPlayer`) false))

(fn `OnPlaybackPercentageChanged`
  (params (PlayingSoundWave :type "SoundWave Object Reference") (PlaybackPercent :type "Float (single-precision)"))
  (`self.PlaybackPercentageChanged` self PlaybackPercent))