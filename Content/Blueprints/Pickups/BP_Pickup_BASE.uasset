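; Base pickup Blueprint, built on capsule and character movement components, that can be launched into the world.
; On BeginPlay it enables tick and holds the PickupComponent's collision off for a short delay before switching it to query-only.
; LaunchPickup applies a mass-independent upward impulse with random sideways X variation to the capsule, then stops character movement shortly afterward.
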(event `self.ReceiveBeginPlay`
  (`self.SetActorTickEnabled` true)
  (`PrimitiveComponent.SetCollisionEnabled` (`self.PickupComponent`) "NoCollision")
  (`KismetSystemLibrary.Delay` 1.0)
  (`PrimitiveComponent.SetCollisionEnabled` (`self.PickupComponent`) "QueryOnly"))

(event `LaunchPickup`
  (`PrimitiveComponent.AddImpulse` (`self.CapsuleComponent`) (+ (`KismetMathLibrary.MakeVector` (`KismetMathLibrary.Conv_IntToDouble` (`KismetMathLibrary.RandomIntegerInRange` -100 100))) (* (0.0 0.0 1.0) 300.0)) "None" true)
  (`KismetSystemLibrary.Delay` 0.2)
  (`MovementComponent.StopMovementImmediately` (`self.CharacterMovement`)))

(fn `UserConstructionScript`)