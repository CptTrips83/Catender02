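; Base Blueprint for wall debris props that get launched when spawned and remove themselves after a set lifespan.
; On BeginPlay the capsule component receives a velocity-change impulse, so its mass does not affect the launch.
; The impulse combines random sideways force on world X and random upward force on Z within configurable ranges, leaving Y at zero.
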(event `self.ReceiveBeginPlay`
  (`PrimitiveComponent.AddImpulse` (`self.CapsuleComponent`) (`self.GetImpulseVelocity`) "None" true)
  (`self.SetLifeSpan` (`self.LifeSpan`)))

(fn `GetImpulseVelocity`
  (returns (Velocity :type "Vector Structure"))
  (return (`KismetMathLibrary.MakeVector` (`KismetMathLibrary.RandomFloatInRange` (`self.MinSideForce`) (`self.MaxSideForce`)) 0.0 (`KismetMathLibrary.RandomFloatInRange` (`self.MinUpForce`) (`self.MaxUpForce`)))))

(fn `UserConstructionScript`)