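; Enemy spawner prop that launches a wave of enemies at its location when world time reaches its start hour.
; It listens to the game mode's day-time component, and a looping timer spawns enemies until the wave count is met.
; Wave size grows with the current day and gets a multiplier every seventh day.
; Every day currently has a wave, and the day-scaled spawn delay function is not used by the timer.
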(event `self.ReceiveBeginPlay`
  (bind _asgm_cat_level (cast `/Game/Blueprints/GameModes/GM_CatLevel` (`GameplayStatics.GetGameMode`)))
  (add `CTWorldDayTimeComponent.OnDayTimeChanged` (`CTGameModeLevel.WorldDayTimeComponent` _asgm_cat_level) (`|CreateDelegate` :!event `DayTimeChanged`)))

(fn `DayHasWave`
  (params (Day :type Integer))
  (returns (DayHasWave :type Boolean))
  (return true))

(fn `DayTimeChanged`
  (params (OldValue :type Integer) (NewValue :type Integer) (OldIsDay :type Boolean) (NewIsDay :type Boolean))
  (if (and (== NewValue (`self.StartHour`)) (`self.DayHasWave` (`self.GetCurrentDay`)))
    (`self.SpawnEnemies`)))

(fn `GetActiveSpawnDelay`
  (returns (SpawnDelay :type "Float (double-precision)"))
  (return (`KismetMathLibrary.FClamp` (- (`self.DefaultSpawnDelay`) (* (`self.SpawnDelayDayModifier`) (`self.GetCurrentDay`))) (`self.MinSpawnDelay`) (`self.DefaultSpawnDelay`))))

(fn `GetCurrentDay`
  (returns (CurrentDay :type Integer))
  (return (`CTWorldDayTimeComponent.CurrentDay` (`CTGameModeLevel.WorldDayTimeComponent` (`self.GetGameMode`)))))

(fn `GetEnemyCountToSpawn`
  (returns (EnemyCount :type Integer))
  (bind _baseenemycounttospawn (`self.BaseEnemyCountToSpawn`))
  (return (`KismetMathLibrary.FCeil` (* (+ _baseenemycounttospawn (`KismetMathLibrary.FCeil` (* _baseenemycounttospawn (* (`self.DailyEnemyCountModifier`) (`self.GetStartDay`))))) (select `bool` (`self.IsHardWave` (`self.GetStartDay`)) :`false` 1.0 :`true` (`self.HardWaveModifier`))))))

(fn `GetSpawnableEnemy`
  (returns (SpawnableEnemyClass :type "/Game/Blueprints/Character/EnemyNPC/BP_Enemy_BASE Class Reference"))
  (return (`self.SpawnableEnemyClass`)))

(fn `GetSpawnDelay`
  (returns (SpawnDelay :type "Float (double-precision)"))
  (return (`self.SpawnDelay`)))

(fn `GetStartDay`
  (returns (StartDay :type Integer))
  (return (`self.GetCurrentDay`)))

(fn `IsHardWave`
  (params (Day :type Integer))
  (returns (IsHardWave :type Boolean))
  (return (== (mod Day 7) 0)))

(fn `SpawnEnemies`
  (locals (EnemyCount :type Integer :default 0))
  (bind _spawndelay (`self.GetSpawnDelay`))
  (bind _returnvalue (`KismetSystemLibrary.K2_SetTimerDelegate` (`|CreateDelegate` :!event `SpawnEnemy`) _spawndelay true false _spawndelay))
  (set `self.TimerHandle` _returnvalue))

(fn `SpawnEnemy`
  (`|SpawnActorFromClass` (`self.GetSpawnableEnemy`) (`KismetMathLibrary.MakeTransform` (`self.K2_GetActorLocation`)) "AlwaysSpawn" "MultiplyWithRoot" null null)
  (bind _result (`/Engine/EditorBlueprintResources/StandardMacros.IncrementInt` (`self.SpawnCounter`))
    (:`  `
      (if (>= _result (`self.GetEnemyCountToSpawn`))
        (`KismetSystemLibrary.K2_ClearAndInvalidateTimerHandle` (`self.TimerHandle`))
        (set `self.SpawnCounter` 0)))))

(fn `UserConstructionScript`)