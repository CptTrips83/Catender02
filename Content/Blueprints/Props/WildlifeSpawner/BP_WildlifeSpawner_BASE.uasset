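; Base wildlife spawner prop that spawns its configured wildlife class at set times of the in-game day.
; On BeginPlay it binds to the day-time change event of GM_CatLevel's WorldDayTimeComponent.
; When the new time is in SpawnHours, it loops over a random spawn amount, calling the game mode's WorldWildlifeComponent to spawn each animal.
; Each spawn lands at the Spawner component's location with a small random X offset.
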(event `self.ReceiveBeginPlay`
  (bind _asgm_cat_level (cast `/Game/Blueprints/GameModes/GM_CatLevel` (`GameplayStatics.GetGameMode`)))
  (add `CTWorldDayTimeComponent.OnDayTimeChanged` (`CTGameModeLevel.WorldDayTimeComponent` _asgm_cat_level) (`|CreateDelegate` :!event `OnDayTimeChanged`)))

(fn `GetSpawnAmount`
  (returns (Amount :type Integer))
  (return (`KismetMathLibrary.RandomIntegerInRange` (`self.MinSpawnAmount`) (`self.MaxSpawnAmount`))))

(fn `OnDayTimeChanged`
  (params (OldValue :type Integer) (NewValue :type Integer) (OldIsDay :type Boolean) (NewIsDay :type Boolean))
  (if (`KismetArrayLibrary.Array_Contains` (`self.SpawnHours`) NewValue)
    (for _ (range (+ (`self.GetSpawnAmount`) 1))
      (`self.SpawnWildlife`))))

(fn `SpawnWildlife`
  (returns (SpawnedWildlife :type "CTWildlife Object Reference"))
  (bind _returnvalue (`CTWorldWildlifeComponent.SpawnWildlife` (`CTGameModeLevel.WorldWildlifeComponent` (`self.GetGameMode`)) (`self.WildlifeClass`) (+ (`SceneComponent.K2_GetComponentLocation` (`self.Spawner`)) (`KismetMathLibrary.MakeVector` (`KismetMathLibrary.RandomFloatInRange` -10.0 10.0)))))
  (return (`|ConvertAsset` _returnvalue)))

(fn `UserConstructionScript`)